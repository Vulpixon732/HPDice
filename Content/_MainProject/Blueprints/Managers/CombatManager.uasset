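; Manager that runs turn-based combat, tracking combatants and handing control to the ExplorationManager whenever the current turn queue empties.
; Initiative comes from each combatant's dice, plus a bonus for the initiator, and feeds an insertion sort that builds the turn order.
; The next round's queue is rolled ahead and promoted when a new round starts, with the player's CombatHUD showing both as overlapping avatar icons.
; EndCombat clears all state and deactivates the manager.
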(event `BeginCombat`
  (`|ExecutionSequence`
    (:`then_0`
      ;[1 1 1] Open Player CombatHUD
      (bind _asbp_player (cast `/Game/_MainProject/Blueprints/Actors/BP_Player` (`GameplayStatics.GetPlayerCharacter` 0)))
      (`/Game/_MainProject/Blueprints/Actors/BP_Player.OpenCombatScreen` _asbp_player))
    (:`then_1`
      ;[1 1 1] Start New Turn if Turn Queue is Empty
      (if (not (`KismetArrayLibrary.Array_IsValidIndex` (`self.CurrentTurnQueue`)))
        (`self.PrepareNewQueue`)
        (`self.StartNewTurn`)))))

(event `EndTurn`
  (`|ExecutionSequence`
    (:`then_0`
      (`KismetArrayLibrary.Array_Remove` (`self.CurrentTurnQueue`)))
    (:`then_1`
      (bind _asbp_player (cast `/Game/_MainProject/Blueprints/Actors/BP_Player` (`GameplayStatics.GetPlayerCharacter` 0)))
      (bind _turnorder (`/Game/_MainProject/Blueprints/Widgets/Combat/CombatHUD.TurnOrder` (`/Game/_MainProject/Blueprints/Actors/BP_Player.CombatHUD` _asbp_player)))
      (bind _currentturnslot (`/Game/_MainProject/Blueprints/Widgets/Combat/TurnOrder/TurnOrder.CurrentTurnSlot` _turnorder))
      (`PanelWidget.ClearChildren` _currentturnslot)
      (`PanelWidget.AddChild` _currentturnslot (`PanelWidget.GetChildAt` (`/Game/_MainProject/Blueprints/Widgets/Combat/TurnOrder/TurnOrder.CurrentTurnOrderBox` _turnorder) 0)))
    (:`then_2`
      (if (> (`KismetArrayLibrary.Array_Length` (`self.CurrentTurnQueue`)) 0)
        (`self.StartNewTurn`)
        (else
          ;[1 1 1] Start New Exploration Turn
          (bind _asmanagers_game_state (cast `/Game/_MainProject/Blueprints/Managers/Managers_GameState` (`GameplayStatics.GetGameState`)))
          (bind _explorationmanager (`/Game/_MainProject/Blueprints/Managers/Managers_GameState.ExplorationManager` _asmanagers_game_state))
          (if (> (`KismetArrayLibrary.Array_Length` (`/Game/_MainProject/Blueprints/Managers/ExplorationManager.TurnQueue` _explorationmanager)) 0)
            (`/Game/_MainProject/Blueprints/Managers/ExplorationManager.StartNewExplorationTurn` _explorationmanager)
            (else
              (`/Game/_MainProject/Blueprints/Managers/ExplorationManager.StartNewExplorationRound` _explorationmanager))))))
    (:`then_3`
      (bind _asbp_player_2 (cast `/Game/_MainProject/Blueprints/Actors/BP_Player` (`GameplayStatics.GetPlayerCharacter` 0)))
      (bind _returnvalue (`PanelWidget.GetChildAt` (`/Game/_MainProject/Blueprints/Widgets/Combat/TurnOrder/TurnOrder.CurrentTurnOrderBox` (`/Game/_MainProject/Blueprints/Widgets/Combat/CombatHUD.TurnOrder` (`/Game/_MainProject/Blueprints/Actors/BP_Player.CombatHUD` _asbp_player_2))) 0))
      (if (`KismetSystemLibrary.IsValid` _returnvalue)
        (bind _ascombatant_turn_icon (cast `/Game/_MainProject/Blueprints/Widgets/Combat/TurnOrder/CombatantTurnIcon` _returnvalue))
        (`VerticalBoxSlot.SetPadding` (`WidgetLayoutLibrary.SlotAsVerticalBoxSlot` _returnvalue) (make `Margin` 0.0 (* (`SizeBox.HeightOverride` (`/Game/_MainProject/Blueprints/Widgets/Combat/TurnOrder/CombatantTurnIcon.IconSizeBox` _ascombatant_turn_icon)) -0.175)))))))

(event `PrepareNewQueue`
  (`|ExecutionSequence`
    (:`then_0`
      ;[1 1 1] Clear Initiative Values
      (`BlueprintMapLibrary.Map_Clear` (`self.NextInitiativeMap`))
      (`BlueprintMapLibrary.Map_Clear` (`self.NextInitiativeIndexMap`)))
    (:`then_1`
      (for _array_element (`self.CombatantsArray`)
        (bind _returnvalue (`|GenericCreateObject` "/Game/_MainProject/Blueprints/Managers/InitiativeWallIndexArray.InitiativeWallIndexArray_C" self))
        (`BlueprintMapLibrary.Map_Add` (`self.NextInitiativeIndexMap`) _array_element _returnvalue)
        (bind _initiative (`self.RollInitiative` _array_element))
        (`BlueprintMapLibrary.Map_Add` (`self.NextInitiativeMap`) _array_element _initiative)))
    (:`then_2`
      (`self.MakeNewTurnQueue`))
    (:`then_3`
      (bind _asbp_player (cast `/Game/_MainProject/Blueprints/Actors/BP_Player` (`GameplayStatics.GetPlayerCharacter` 0)))
      (bind _nextturnorderbox (`/Game/_MainProject/Blueprints/Widgets/Combat/TurnOrder/TurnOrder.NextTurnOrderBox` (`/Game/_MainProject/Blueprints/Widgets/Combat/CombatHUD.TurnOrder` (`/Game/_MainProject/Blueprints/Actors/BP_Player.CombatHUD` _asbp_player))))
      (`PanelWidget.ClearChildren` _nextturnorderbox)
      (for _array_element_2 (`self.NextTurnQueue`)
        (bind _ascombat_character_base (cast `/Game/_MainProject/Blueprints/Actors/CombatCharacterBase` _array_element_2))
        (bind _returnvalue_2 (`|CreateWidget` "/Game/_MainProject/Blueprints/Widgets/Combat/TurnOrder/CombatantTurnIcon.CombatantTurnIcon_C" null (`/Game/_MainProject/Blueprints/Actors/CombatCharacterBase.TurnAvatar` _ascombat_character_base) _array_element_2))
        (`PanelWidget.AddChild` _nextturnorderbox _returnvalue_2))
      (for (_array_element_3 _array_index) (`PanelWidget.GetAllChildren` _nextturnorderbox)
        (bind _ascombatant_turn_icon (cast `/Game/_MainProject/Blueprints/Widgets/Combat/TurnOrder/CombatantTurnIcon` _array_element_3))
        (if (> _array_index 0)
          (`VerticalBoxSlot.SetPadding` (`WidgetLayoutLibrary.SlotAsVerticalBoxSlot` _array_element_3) (make `Margin` 0.0 (* (`SizeBox.HeightOverride` (`/Game/_MainProject/Blueprints/Widgets/Combat/TurnOrder/CombatantTurnIcon.IconSizeBox` _ascombatant_turn_icon)) -0.25)))
          (else
            (`VerticalBoxSlot.SetPadding` (`WidgetLayoutLibrary.SlotAsVerticalBoxSlot` _array_element_3) (make `Margin` 0.0 (* (`SizeBox.HeightOverride` (`/Game/_MainProject/Blueprints/Widgets/Combat/TurnOrder/CombatantTurnIcon.IconSizeBox` _ascombatant_turn_icon)) -0.175)))))))))

(event `StartNewTurn`
  (bind _output (`|GetArrayItem` (`self.CurrentTurnQueue`)))
  (if (not (> (`KismetArrayLibrary.Array_Length` (`self.CurrentTurnQueue`)) 0))
    (set `self.CurrentInitiativeIndexMap` (`self.NextInitiativeIndexMap`))
    (set `self.CurrentTurnQueue` (`self.NextTurnQueue`))
    (set `self.CurrentInitiativeMap` (`self.NextInitiativeMap`))
    (bind _asbp_player (cast `/Game/_MainProject/Blueprints/Actors/BP_Player` (`GameplayStatics.GetPlayerCharacter` 0)))
    (bind _turnorder (`/Game/_MainProject/Blueprints/Widgets/Combat/CombatHUD.TurnOrder` (`/Game/_MainProject/Blueprints/Actors/BP_Player.CombatHUD` _asbp_player)))
    (bind _currentturnorderbox (`/Game/_MainProject/Blueprints/Widgets/Combat/TurnOrder/TurnOrder.CurrentTurnOrderBox` _turnorder))
    (`PanelWidget.ClearChildren` _currentturnorderbox)
    (bind _currentturnslot (`/Game/_MainProject/Blueprints/Widgets/Combat/TurnOrder/TurnOrder.CurrentTurnSlot` _turnorder))
    (bind _nextturnorderbox (`/Game/_MainProject/Blueprints/Widgets/Combat/TurnOrder/TurnOrder.NextTurnOrderBox` _turnorder))
    (`PanelWidget.AddChild` _currentturnslot (`PanelWidget.GetChildAt` _nextturnorderbox 0))
    (bind _ascombatant_turn_icon (cast `/Game/_MainProject/Blueprints/Widgets/Combat/TurnOrder/CombatantTurnIcon` (`PanelWidget.GetChildAt` _currentturnslot 0)))
    (`VerticalBoxSlot.SetPadding` (`WidgetLayoutLibrary.SlotAsVerticalBoxSlot` _currentturnslot) (make `Margin` 0.0 (* (`SizeBox.HeightOverride` (`/Game/_MainProject/Blueprints/Widgets/Combat/TurnOrder/CombatantTurnIcon.IconSizeBox` _ascombatant_turn_icon)) -0.175)))
    (while (> (`KismetArrayLibrary.Array_Length` (`PanelWidget.GetAllChildren` _nextturnorderbox)) 0)
      (`VerticalBox.AddChildToVerticalBox` _currentturnorderbox (`PanelWidget.GetChildAt` _nextturnorderbox 0)))
    (for (_array_element _array_index) (`PanelWidget.GetAllChildren` _currentturnorderbox)
      (bind _ascombatant_turn_icon_2 (cast `/Game/_MainProject/Blueprints/Widgets/Combat/TurnOrder/CombatantTurnIcon` _array_element))
      (if (> _array_index 0)
        (`VerticalBoxSlot.SetPadding` (`WidgetLayoutLibrary.SlotAsVerticalBoxSlot` _array_element) (make `Margin` 0.0 (* (`SizeBox.HeightOverride` (`/Game/_MainProject/Blueprints/Widgets/Combat/TurnOrder/CombatantTurnIcon.IconSizeBox` _ascombatant_turn_icon_2)) -0.25)))
        (else
          (`VerticalBoxSlot.SetPadding` (`WidgetLayoutLibrary.SlotAsVerticalBoxSlot` _array_element) (make `Margin` 0.0 (* (`SizeBox.HeightOverride` (`/Game/_MainProject/Blueprints/Widgets/Combat/TurnOrder/CombatantTurnIcon.IconSizeBox` _ascombatant_turn_icon_2)) -0.175))))))
    (`self.PrepareNewQueue`))
  (message `/Game/_MainProject/Blueprints/Managers/CombatInterface.StartTurn` _output)
  (`KismetSystemLibrary.PrintString` (`KismetTextLibrary.Conv_TextToString` (`|FormatText` "///Starting CombatTurn: {Actor}" _output))))

(event `EndCombat`
  (`|ExecutionSequence`
    (:`then_0`
      (`KismetArrayLibrary.Array_Clear` (`self.CombatantsArray`)))
    (:`then_1`
      (`KismetArrayLibrary.Array_Clear` (`self.NextTurnQueue`)))
    (:`then_2`
      (`KismetArrayLibrary.Array_Clear` (`self.CurrentTurnQueue`)))
    (:`then_3`
      (`BlueprintMapLibrary.Map_Clear` (`self.NextInitiativeMap`)))
    (:`then_4`
      (`BlueprintMapLibrary.Map_Clear` (`self.CurrentInitiativeMap`)))
    (:`then_5`
      (`BlueprintMapLibrary.Map_Clear` (`self.NextInitiativeIndexMap`)))
    (:`then_6`
      (`BlueprintMapLibrary.Map_Clear` (`self.CurrentInitiativeIndexMap`)))
    (:`then_7`
      (set `self.Initiator` null))
    (:`then_8`
      (bind _asbp_player (cast `/Game/_MainProject/Blueprints/Actors/BP_Player` (`GameplayStatics.GetPlayerCharacter` 0)))
      (`/Game/_MainProject/Blueprints/Actors/BP_Player.EndCombatPlayer` _asbp_player))
    (:`then_9`
      (`self.Deactivate` self))))

(fn `IsActorInCombat`
  (params (ActorToFind :type "/Game/_MainProject/Blueprints/Actors/CombatCharacterBase Object Reference"))
  (returns (IsInCombat :type Boolean))
  (return (`KismetArrayLibrary.Array_Contains` (`self.CombatantsArray`) ActorToFind)))

(fn `MakeNewTurnQueue`
  (locals (TargetIndex :type Integer) (AddedIndex :type Integer) (ItemAdded :type Boolean))
  (for _array_element (`self.CombatantsArray`)
    (if (`KismetArrayLibrary.Array_IsValidIndex` (`self.NextTurnQueue`))
      (`|ExecutionSequence`
        (:`then_0`
          ;[1 1 1] Add New Actor to Turn Queue
          (for (_array_element_2 _array_index) (`self.NextTurnQueue`)
            (if (> _array_index 0)
              (if (<= (`BlueprintMapLibrary.Map_Find` (`self.NextInitiativeMap`) _array_element_2) (`BlueprintMapLibrary.Map_Find` (`self.NextInitiativeMap`) _array_element))
                (set `local.TargetIndex` _array_index)
                (bind _returnvalue (`KismetArrayLibrary.Array_AddUnique` (`self.NextTurnQueue`) _array_element))
                (set `local.AddedIndex` _returnvalue)
                (set `local.ItemAdded` true)
                (break)))))
        (:`then_1`
          ;[1 1 1] Add new Actor at last index to Listen Queue
          (if (not (`local.ItemAdded`))
            (bind _returnvalue_2 (`KismetArrayLibrary.Array_AddUnique` (`self.NextTurnQueue`) _array_element))
            (bind _output_get (set `local.AddedIndex` _returnvalue_2))
            (set `local.TargetIndex` _output_get)))
        (:`then_2`
          ;[1 1 1] Swap Widgets in Queue to adjust Priority of new item
          (while (> (`local.AddedIndex`) (`local.TargetIndex`))
            (`KismetArrayLibrary.Array_Swap` (`self.NextTurnQueue`) (`local.AddedIndex`) (- (`local.AddedIndex`) 1))
            (`/Engine/EditorBlueprintResources/StandardMacros.DecrementInt` (`local.AddedIndex`)))))
      (else
        ;[1 1 1] Add first Actor to Queue
        (`KismetArrayLibrary.Array_AddUnique` (`self.NextTurnQueue`) _array_element)))))

(fn `RollInitiative`
  (params (Actor :type "Actor Object Reference"))
  (returns (Initiative :type Integer))
  (locals (TmpDiceArray :type "Array of /Game/_MainProject/Blueprints/Widgets/Dice/Dice Object Reference") (TmpInitiative :type Integer))
  (bind _value (`BlueprintMapLibrary.Map_Find` (`self.NextInitiativeIndexMap`) (`local.Actor`)))
  (if (== Actor (`self.Initiator`))
    (set `local.TmpInitiative` 6) ; Bonus Initiative for Initiating Combat
    (set `self.Initiator` null))
  (bind _ascombat_character_base (cast `/Game/_MainProject/Blueprints/Actors/CombatCharacterBase` Actor))
  (set `local.TmpDiceArray` (`/Game/_MainProject/Blueprints/Actors/CombatCharacterBase.DiceArray` _ascombat_character_base))
  (bind (_returndicecount _filtereddicearray) (`/Game/_MainProject/Blueprints/FunctionLibrary.GetDicesInSlot` (`local.TmpDiceArray`) "NewEnumerator5"))
  (if (> _returndicecount 0)
    (for _array_element _filtereddicearray
      (if (`|EnumInequality` (`/Game/_MainProject/Blueprints/Widgets/Dice/Dice.DiceType` _array_element) "NewEnumerator4")
        (`/Game/_MainProject/Blueprints/Widgets/Dice/Dice.RollRandom` _array_element)
        (set `local.TmpInitiative` (+ (`local.TmpInitiative`) (`/Game/_MainProject/Blueprints/Widgets/Dice/Dice.RolledValue` _array_element)))
        (else
          (bind (_highestvalue _wallindex) (`/Game/_MainProject/Blueprints/Widgets/Dice/Dice.Get Highest Value` _array_element))
          (`/Game/_MainProject/Blueprints/Widgets/Dice/Dice.SetCurrentWallByIndex` _array_element _wallindex)
          (set `local.TmpInitiative` (+ (`local.TmpInitiative`) _highestvalue))))
      (`KismetArrayLibrary.Array_Add` (`/Game/_MainProject/Blueprints/Managers/InitiativeWallIndexArray.DiceReferenceArray` _value) _array_element)
      (`KismetArrayLibrary.Array_Add` (`/Game/_MainProject/Blueprints/Managers/InitiativeWallIndexArray.IndexArray` _value) (`/Game/_MainProject/Blueprints/Widgets/Dice/Dice.RolledWallIndex` _array_element))))
  (return (`local.TmpInitiative`)))