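; Game state Blueprint that acts as a hub for turn-based play, forwarding turn events to separate exploration and combat managers.
; It starts an exploration round on BeginPlay.
; BeginCombat activates the combat manager, registers initiator and target as combatants, removes both from the exploration turn queue, then starts combat.
; End-of-turn events for combat and exploration pass straight through to their respective managers.
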(event `self.ReceiveBeginPlay`
  (`|ExecutionSequence`
    (:`then_0`
      (`/Game/_MainProject/Blueprints/Managers/ExplorationManager.StartNewExplorationRound` (`self.ExplorationManager`)))))

(event `BeginCombat`
  (params (Initiator :type "/Game/_MainProject/Blueprints/Actors/CombatCharacterBase Object Reference") (TargetVictim :type "/Game/_MainProject/Blueprints/Actors/CombatCharacterBase Object Reference"))
  (bind _combatmanager (`self.CombatManager`))
  (bind _turnqueue (`/Game/_MainProject/Blueprints/Managers/ExplorationManager.TurnQueue` (`self.ExplorationManager`)))
  (bind _combatantsarray (`/Game/_MainProject/Blueprints/Managers/CombatManager.CombatantsArray` _combatmanager))
  (`ActorComponent.Activate` (`self.CombatManager`) false)
  (`KismetArrayLibrary.Array_AddUnique` _combatantsarray Initiator)
  (`KismetArrayLibrary.Array_AddUnique` _combatantsarray TargetVictim)
  (`KismetArrayLibrary.Array_RemoveItem` _turnqueue Initiator)
  (`KismetArrayLibrary.Array_RemoveItem` _turnqueue TargetVictim)
  (set `/Game/_MainProject/Blueprints/Managers/CombatManager.Initiator` Initiator _combatmanager)
  (`/Game/_MainProject/Blueprints/Managers/CombatManager.BeginCombat` _combatmanager))

(event `EndCombatTurn`
  (`/Game/_MainProject/Blueprints/Managers/CombatManager.EndTurn` (`self.CombatManager`)))

(event `EndExplorationTurn`
  (`/Game/_MainProject/Blueprints/Managers/ExplorationManager.EndCurrentExplorationTurn` (`self.ExplorationManager`)))

(fn `UserConstructionScript`)