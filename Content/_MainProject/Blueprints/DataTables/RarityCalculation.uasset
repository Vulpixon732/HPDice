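; Blueprint helper functions that roll a Common, Uncommon or Rare result from a seeded stream within a lowest-to-highest rarity range.
; Caller-owned chances, passed by reference, act as cumulative thresholds; UseBaseChance affects only the range bounds.
; Optional bad-luck protection shifts chance from Common to higher rarities not rolled, while ResetChance restores selected tiers to base and redistributes the difference.
; Rolls and chance changes print debug text.
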(fn `GetRandomRarity`
  (params (LowestRarity :type "/Game/_MainProject/Blueprints/Enumerations/EnumRarity Enum" :default "NewEnumerator0") (HighestRarity :type "/Game/_MainProject/Blueprints/Enumerations/EnumRarity Enum" :default "NewEnumerator2") (ResetChanceForOutput :type Boolean :default true) (IncreaseLuckAfter :type Boolean :default true) (UseBaseChance :type Boolean) (Seed :type "RandomStream Structure (by ref)") (CurrentCommonChance_R :type "Float (double-precision) (by ref)") (CurrentUncommonChance_R :type "Float (double-precision) (by ref)") (CurrentRareChance_R :type "Float (double-precision) (by ref)") (WorldContextObject :type "Object Object Reference"))
  (returns (OutputRarity :type "/Game/_MainProject/Blueprints/Enumerations/EnumRarity Enum"))
  (locals (Min :type "Float (double-precision)") (Max :type "Float (double-precision)" :default 1.0) (Result :type "Float (double-precision)"))
  (switch `/Game/_MainProject/Blueprints/Enumerations/EnumRarity` LowestRarity
    (:`NewEnumerator0`
      (set `local.Min` 0.0))
    (:`NewEnumerator1`
      (set `local.Min` (+ (`KismetMathLibrary.SelectFloat` (`self.BaseCommonChance`) (`local.CurrentCommonChance_R`) UseBaseChance) 1e-06)))
    (:`NewEnumerator2`
      (set `local.Min` (+ (`KismetMathLibrary.SelectFloat` (`self.BaseCommonChance`) (`local.CurrentCommonChance_R`) UseBaseChance) (`KismetMathLibrary.SelectFloat` (`self.BaseUncommonChance`) (`local.CurrentUncommonChance_R`) UseBaseChance) 1e-06))))
  (switch `/Game/_MainProject/Blueprints/Enumerations/EnumRarity` HighestRarity
    (:`NewEnumerator0`
      (set `local.Max` (`KismetMathLibrary.SelectFloat` (`self.BaseCommonChance`) (`local.CurrentCommonChance_R`) UseBaseChance)))
    (:`NewEnumerator1`
      (set `local.Max` (+ (`KismetMathLibrary.SelectFloat` (`self.BaseCommonChance`) (`local.CurrentCommonChance_R`) UseBaseChance) (`KismetMathLibrary.SelectFloat` (`self.BaseUncommonChance`) (`local.CurrentUncommonChance_R`) UseBaseChance))))
    (:`NewEnumerator2`
      (set `local.Max` (+ (`KismetMathLibrary.SelectFloat` (`self.BaseCommonChance`) (`local.CurrentCommonChance_R`) UseBaseChance) (`KismetMathLibrary.SelectFloat` (`self.BaseUncommonChance`) (`local.CurrentUncommonChance_R`) UseBaseChance) (`KismetMathLibrary.SelectFloat` (`self.BaseRareChance`) (`local.CurrentRareChance_R`) UseBaseChance)))))
  (if (<= (`local.Min`) (`local.Max`))
    (set `local.Result` (`KismetMathLibrary.RandomFloatInRangeFromStream` (`local.Min`) (`local.Max`) Seed))
    (if (<= (`local.Result`) (`local.CurrentCommonChance_R`))
      ;[1 1 1] RESULT - COMMON
      (`KismetSystemLibrary.PrintText` WorldContextObject (`|FormatText` ">>GetRandomRarity \nBase Chance Used: {Luck} \nGenerated Value: {Result} \nOutput Rarity: Common \n<<" (`local.Result`) (`local.UseBaseChance`)))
      (if IncreaseLuckAfter
        (`|ExecutionSequence`
          (:`then_0`
            (`self.IncreaseUncommonChance` WorldContextObject (`local.CurrentCommonChance_R`) (`local.CurrentUncommonChance_R`)))
          (:`then_1`
            (`self.IncreaseRareChance` WorldContextObject (`local.CurrentCommonChance_R`) (`local.CurrentRareChance_R`)))
          (:`then_2`
            (return "NewEnumerator0")))
        (else
          (return "NewEnumerator0")))
      (else
        ;[0.4133 0.8386 1] RESULT - UNCOMMON
        (if (<= (`local.Result`) (+ (`local.CurrentCommonChance_R`) (`local.CurrentUncommonChance_R`)))
          (`KismetSystemLibrary.PrintText` (`local.WorldContextObject`) (`|FormatText` ">>GetRandomRarity \nBase Chance Used: {Luck} \nGenerated Value: {Result} \nOutput Rarity: Uncommon \n<<" (`local.Result`) (`local.UseBaseChance`)))
          (if ResetChanceForOutput
            (`self.ResetChance` false true false (`local.CurrentCommonChance_R`) (`local.CurrentUncommonChance_R`) (`local.CurrentRareChance_R`) WorldContextObject))
          (if IncreaseLuckAfter
            (`self.IncreaseRareChance` (`local.WorldContextObject`) (`local.CurrentCommonChance_R`) (`local.CurrentRareChance_R`)))
          (return "NewEnumerator1")
          (else
            ;[1 0.9009 0.1521] RESULT - RARE
            (`KismetSystemLibrary.PrintText` (`local.WorldContextObject`) (`|FormatText` ">>GetRandomRarity \nBase Chance Used: {Luck} \nGenerated Value: {Result} \nOutput Rarity: Rare \n<<" (`local.Result`) (`local.UseBaseChance`)))
            (if ResetChanceForOutput
              (`self.ResetChance` false false true (`local.CurrentCommonChance_R`) (`local.CurrentUncommonChance_R`) (`local.CurrentRareChance_R`) (`local.WorldContextObject`)))
            (if IncreaseLuckAfter
              (`self.IncreaseUncommonChance` (`local.WorldContextObject`) (`local.CurrentCommonChance_R`) (`local.CurrentUncommonChance_R`)))
            (return "NewEnumerator2")))))
    (else
      ;[1 0.08333 0.08333] ERROR - Invalid Rarity Range
      (`KismetSystemLibrary.PrintString` null (`KismetTextLibrary.Conv_TextToString` (`|FormatText` "/// \nERROR \nSource: {SourceBlueprint} \nReason: Invalid Rarity Range \n///" (`KismetSystemLibrary.GetDisplayName` self))) true true (struct :`R` 1.0 :`A` 1.0) 10.0))))

(fn `IncreaseRareChance`
  (params (WorldContextObject :type "Object Object Reference") (CurrentCommonChanceR :type "Float (double-precision) (by ref)") (CurrentRareChanceR :type "Float (double-precision) (by ref)"))
  (`KismetSystemLibrary.PrintText` WorldContextObject (`|FormatText` ">>>Increasing Rare Chance \nPrevious Common Chance: {PreviousC} \nPrevious Rare Chance: {PreviousUC} \n" (`local.CurrentCommonChanceR`) (`local.CurrentRareChanceR`)))
  (`|VariableSetRef` (`local.CurrentRareChanceR`) (+ (`local.CurrentRareChanceR`) (`self.BaseRareChanceIncrease`)))
  (`|VariableSetRef` (`local.CurrentCommonChanceR`) (- (`local.CurrentCommonChanceR`) (`self.BaseRareChanceIncrease`)))
  (`KismetSystemLibrary.PrintText` WorldContextObject (`|FormatText` "--- \nCurrent Common Chance: {PreviousC} (-{increment}) \nCurrent Rare Chance: {PreviousUC} (+{increment}) \n<<<" (`local.CurrentCommonChanceR`) (`self.BaseRareChanceIncrease`) (`local.CurrentRareChanceR`))))

(fn `IncreaseUncommonChance`
  (params (WorldContextObject :type "Object Object Reference") (CurrentCommonChanceR :type "Float (double-precision) (by ref)") (CurrentUncommonChanceR :type "Float (double-precision) (by ref)"))
  (`KismetSystemLibrary.PrintText` WorldContextObject (`|FormatText` ">>>Increasing Uncommon Chance \nPrevious Common Chance: {PreviousC} \nPrevious Uncommon Chance: {PreviousUC} \n---" (`local.CurrentUncommonChanceR`) (`local.CurrentCommonChanceR`)))
  (`|VariableSetRef` (`local.CurrentUncommonChanceR`) (+ (`local.CurrentUncommonChanceR`) (`self.BaseUncommonChanceIncrease`)))
  (`|VariableSetRef` (`local.CurrentCommonChanceR`) (- (`local.CurrentCommonChanceR`) (`self.BaseUncommonChanceIncrease`)))
  (`KismetSystemLibrary.PrintText` (`local.WorldContextObject`) (`|FormatText` "--- \nCurrent Common Chance: {PreviousC} (-{increment}) \nCurrent Uncommon Chance: {PreviousUC} (+{increment}) \n<<<" (`local.CurrentCommonChanceR`) (`self.BaseUncommonChanceIncrease`) (`local.CurrentUncommonChanceR`))))

(fn `ResetChance`
  (params (Common :type Boolean) (Uncommon :type Boolean) (Rare :type Boolean) (CurrentCommonChance_R :type "Float (double-precision) (by ref)") (CurrentUncommonChance_R :type "Float (double-precision) (by ref)") (CurrentRareChance_R :type "Float (double-precision) (by ref)") (WorldContextObject :type "Object Object Reference"))
  (locals (Difference :type "Float (double-precision)"))
  (bind _currentrarechance_r (`local.CurrentRareChance_R`))
  (bind _currentuncommonchance_r (`local.CurrentUncommonChance_R`))
  (bind _currentcommonchance_r (`local.CurrentCommonChance_R`))
  (bind _currentcommonchance_r_2 (`local.CurrentCommonChance_R`))
  (bind _currentcommonchance_r_3 (`local.CurrentCommonChance_R`))
  (`|ExecutionSequence`
    (:`then_0`
      (`KismetSystemLibrary.PrintText` WorldContextObject (`|FormatText` ">>Reseting Rarity Chance for: \nCommon - {CB} \nUncommon - {UCB} \nRare - {RB} \n \nPrevious Common Chance: {C} \nPrevious Uncommon Chance: {UC} \nPrevious Rare Chance: {RC} \n---" (`local.Common`) (`local.Uncommon`) (`local.Rare`) (`local.CurrentCommonChance_R`) (`local.CurrentUncommonChance_R`) (`local.CurrentRareChance_R`))))
    (:`then_1`
      (if (`local.Common`)
        ;[1 1 1] TRUE - COMMON
        (set `local.Difference` (- (`local.CurrentCommonChance_R`) (`self.BaseCommonChance`))) ; Compare chance difference for upcoming value normalization
        (`|VariableSetRef` (`local.CurrentCommonChance_R`) (`self.BaseCommonChance`))
        (if (and (`local.Uncommon`) (`local.Rare`))
          ;;[1 1 1] True - Uncommon and Rare chance Reset
          (`|VariableSetRef` (`local.CurrentUncommonChance_R`) (`self.BaseUncommonChance`))
          (`|VariableSetRef` (`local.CurrentRareChance_R`) (`self.BaseRareChance`))
          (elif (`local.Uncommon`)
            ;;[1 1 1] True - Reset Uncommon Chance, add Difference to Rare
            (set `local.Difference` (+ (`local.Difference`) (- (`self.BaseUncommonChance`) (`local.CurrentUncommonChance_R`))))
            (`|VariableSetRef` (`local.CurrentUncommonChance_R`) (`self.BaseUncommonChance`))
            (`|VariableSetRef` _currentrarechance_r (+ _currentrarechance_r (`local.Difference`)))
            (elif (`local.Rare`)
              ;;[1 1 1] True - Reset Rare Chance, add Difference to Uncommon
              (set `local.Difference` (+ (`local.Difference`) (- (`self.BaseRareChance`) (`local.CurrentRareChance_R`))))
              (`|VariableSetRef` (`local.CurrentRareChance_R`) (`self.BaseRareChance`))
              (`|VariableSetRef` _currentuncommonchance_r (+ _currentuncommonchance_r (`local.Difference`)))
              (else
                ;;[1 1 1] False - Add normalized difference to Uncommon and Rare
                (`|VariableSetRef` (`local.CurrentUncommonChance_R`) (+ (`local.CurrentUncommonChance_R`) (* (/ (`self.BaseUncommonChanceIncrease`) (+ (`self.BaseUncommonChanceIncrease`) (`self.BaseRareChanceIncrease`))) (`local.Difference`))))
                (`|VariableSetRef` (`local.CurrentRareChance_R`) (+ (`local.CurrentRareChance_R`) (* (/ (`self.BaseRareChanceIncrease`) (+ (`self.BaseUncommonChanceIncrease`) (`self.BaseRareChanceIncrease`))) (`local.Difference`))))))))
        (else
          ;[1 1 1] FALSE - Check for Uncommon and Rare Reset
          (if (and (`local.Uncommon`) (`local.Rare`))
            ;;[1 1 1] True - Reset both and add difference to Common
            (set `local.Difference` (- (`local.CurrentUncommonChance_R`) (`self.BaseUncommonChance`)))
            (`|VariableSetRef` (`local.CurrentUncommonChance_R`) (`self.BaseUncommonChance`))
            (set `local.Difference` (+ (`local.Difference`) (- (`local.CurrentRareChance_R`) (`self.BaseRareChance`))))
            (`|VariableSetRef` (`local.CurrentRareChance_R`) (`self.BaseRareChance`))
            (`|VariableSetRef` _currentcommonchance_r_2 (+ _currentcommonchance_r_2 (`local.Difference`)))
            (elif (`local.Uncommon`)
              ;;[1 1 1] True - Reset Uncommon, add difference to Common
              (set `local.Difference` (- (`local.CurrentUncommonChance_R`) (`self.BaseUncommonChance`)))
              (`|VariableSetRef` (`local.CurrentUncommonChance_R`) (`self.BaseUncommonChance`))
              (`|VariableSetRef` _currentcommonchance_r_3 (+ _currentcommonchance_r_3 (`local.Difference`)))
              (elif (`local.Rare`)
                ;;[1 1 1] True - Reset Rare, add difference to Common
                (set `local.Difference` (- (`local.CurrentRareChance_R`) (`self.BaseRareChance`)))
                (`|VariableSetRef` (`local.CurrentRareChance_R`) (`self.BaseRareChance`))
                (`|VariableSetRef` _currentcommonchance_r (+ _currentcommonchance_r (`local.Difference`)))
                (else
                  (`KismetSystemLibrary.PrintText` WorldContextObject ">>> WARNING - ResetChance should not be called with False on each Bool Input <<< \n---" true true (struct :`R` 1.0 :`G` 0.831897 :`A` 1.0)))))))))
    (:`then_2`
      (`KismetSystemLibrary.PrintText` WorldContextObject (`|FormatText` "Current Common Chance: {C} \nCurrent Uncommon Chance: {UC} \nCurrent Rare Chance: {RC} \n---" (`local.CurrentCommonChance_R`) (`local.CurrentUncommonChance_R`) (`local.CurrentRareChance_R`))))))

(fn `SetupCurrentChance`
  (params (Common :type "Float (double-precision) (by ref)") (Uncommon :type "Float (double-precision) (by ref)") (Rare :type "Float (double-precision) (by ref)"))
  (`|ExecutionSequence`
    (:`then_0`
      (`|VariableSetRef` Common (`self.BaseCommonChance`)))
    (:`then_1`
      (`|VariableSetRef` Uncommon (`self.BaseUncommonChance`)))
    (:`then_2`
      (`|VariableSetRef` Rare (`self.BaseRareChance`)))))