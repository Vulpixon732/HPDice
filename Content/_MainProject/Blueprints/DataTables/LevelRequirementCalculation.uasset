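; LevelRequirementCalculation resolves level-ups from a level and current EXP, returning EXP within the level, the requirement and the level-up count.
; Each level's requirement grows by the next ExpRaisePerLevel entry, wrapping by modulo, and accumulates into a running total.
; While EXP meets that total, ValidateEXP increments the level and re-enters the loop for just that level.
; The summed ExpPerRepeat value is never read.
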(fn `ValidateEXP`
  (params (Level :type "Integer (by ref)") (CurrentEXP :type "Integer (by ref)"))
  (returns (PlayerEXP :type Integer) (RequiredEXP :type Integer) (LevelUpInstances :type Integer))
  (locals (ExpNeeded :type Integer :default 0) (LevelUps :type Integer) (ExpPerRepeat :type Integer) (LoopFirstIndex :type Integer :default 1) (LoopLastIndex :type Integer) (ExpTotal :type Integer :default 0) (LevelsTillRepeat :type Integer :default 6))
  (set `local.LevelsTillRepeat` (`KismetArrayLibrary.Array_Length` (`self.ExpRaisePerLevel`)))
  (bind _output_get (set `local.LoopLastIndex` Level))
  (for _array_element (`self.ExpRaisePerLevel`)
    (set `local.ExpPerRepeat` (+ (`local.ExpPerRepeat`) _array_element)))
  (for _index (range (`local.LoopFirstIndex`) (+ _output_get 1)) :!label _label
    ;[1 1 1] GetValueFromExpRaisePerLevel
    (bind _output_get_2 (set `local.ExpNeeded` (+ (`local.ExpNeeded`) (`|GetArrayItem` (`self.ExpRaisePerLevel`) (mod (- _index 1) (`local.LevelsTillRepeat`))))))
    ;[1 1 1] Total Exp for all previous levels + previous
    (set `local.ExpTotal` (+ (`local.ExpTotal`) _output_get_2)))
  (if (>= CurrentEXP (`local.ExpTotal`))
    (bind _result (`/Engine/EditorBlueprintResources/StandardMacros.IncrementInt` Level)
      (:`  `
        (`/Engine/EditorBlueprintResources/StandardMacros.IncrementInt` (`local.LevelUps`)
          (:`  `
            (set `local.LoopFirstIndex` _result)
            (set `local.LoopLastIndex` _result)
            (goto _label)))))
    (else
      (return (+ (- CurrentEXP (`local.ExpTotal`)) (`local.ExpNeeded`)) (`local.ExpNeeded`) (`local.LevelUps`)))))