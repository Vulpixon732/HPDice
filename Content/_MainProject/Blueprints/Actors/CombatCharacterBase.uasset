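; CombatCharacterBase is the shared base for characters taking part in exploration and combat turns.
; On BeginPlay it creates dice widgets from a preset class array into DiceArray.
; Spending all moves ends the exploration turn, notifying BP_Player (if self is one) and Managers_GameState, which also receives combat turn endings.
; KillActor removes the character from active CombatManager and DamageManager lists before destroying it.
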(event `self.ReceiveBeginPlay`
  ;[1 1 1] Create Dices in Preset
  (if (`KismetArrayLibrary.Array_IsValidIndex` (`self.DiceArrayPreset`))
    (for _array_element (`self.DiceArrayPreset`)
      (bind _returnvalue (`|CreateWidget` :`Class` _array_element :`Owner` self))
      (`KismetArrayLibrary.Array_Add` (`self.DiceArray`) _returnvalue))))

(event `ReduceMovesLeft`
  (params (ReduceBy :type Integer :default 1))
  (bind _output_get (set `self.MovesLeft` (- (`self.MovesLeft`) ReduceBy)))
  (if (<= _output_get 0)
    (`self.EndExplorationTurn`)))

(event `EndExplorationTurn`
  (`|ExecutionSequence`
    (:`then_0`
      (bind _asbp_player (cast `/Game/_MainProject/Blueprints/Actors/BP_Player` self))
      (`/Game/_MainProject/Blueprints/Actors/BP_Player.PlayerEndOfExplorationTurn` _asbp_player))
    (:`then_1`
      (bind _asmanagers_game_state (cast `/Game/_MainProject/Blueprints/GameModes/Managers/Managers_GameState` (`GameplayStatics.GetGameState`)))
      (`/Game/_MainProject/Blueprints/GameModes/Managers/Managers_GameState.EndExplorationTurn` _asmanagers_game_state))))

(event `KillActor`
  (`|ExecutionSequence`
    (:`then_0`
      (bind _asmanagers_game_state (cast `/Game/_MainProject/Blueprints/GameModes/Managers/Managers_GameState` (`GameplayStatics.GetGameState`)))
      (`|ExecutionSequence`
        (:`then_0`
          (bind _combatmanager (`/Game/_MainProject/Blueprints/GameModes/Managers/Managers_GameState.CombatManager` _asmanagers_game_state))
          (if (`ActorComponent.IsActive` _combatmanager)
            (`KismetArrayLibrary.Array_RemoveItem` (`/Game/_MainProject/Blueprints/GameModes/Managers/CombatManager.CombatantsArray` _combatmanager) self)))
        (:`then_1`
          (bind _damagemanager (`/Game/_MainProject/Blueprints/GameModes/Managers/Managers_GameState.DamageManager` _asmanagers_game_state))
          (if (`ActorComponent.IsActive` _damagemanager)
            (`KismetArrayLibrary.Array_RemoveItem` (`/Game/_MainProject/Blueprints/GameModes/Managers/DamageManager.Targets` _damagemanager) self)))))
    (:`then_1`
      (`self.K2_DestroyActor`))))

(event `EndCombatTurn`
  (`|ExecutionSequence`
    (:`then_1`
      (bind _asmanagers_game_state (cast `/Game/_MainProject/Blueprints/GameModes/Managers/Managers_GameState` (`GameplayStatics.GetGameState`)))
      (`/Game/_MainProject/Blueprints/GameModes/Managers/Managers_GameState.EndCombatTurn` _asmanagers_game_state))))

(fn `UserConstructionScript`)