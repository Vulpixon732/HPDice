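; Player character for a turn-based, grid-style dungeon crawler with dice, handling input, exploration and combat turns, and HUD switching.
; Timelines lerp 90-degree turns and fixed-distance steps under an input lock; steps are trace-checked, cost a move even when blocked, and are disabled during combat.
; After a combat turn, a forward trace loads the HUD of the faced hostile combatant.
; BeginPlay creates both HUDs, registers with the GameMode and refreshes EXP; level-up only prints.
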(event `Rotate`
  (params (Rotation :type "Float (double-precision)"))
  (bind _returnvalue (`GameplayStatics.GetPlayerController` 0))
  (bind _yaw (.yaw (`self.K2_GetActorRotation`)))
  ;[1 1 1] Rotate Camera and Character
  (set `self.InputLock` true)
  (`/Engine/EditorBlueprintResources/StandardMacros.DoOnce` false :!label _label
    (:`Completed`
      (bind _output_get (set `self.StartYawRotation` _yaw))
      (bind _output_get_2 (set `self.EndYawRotation` (+ _yaw Rotation)))
      (bind (_direction _lerp_alpha) (`Timeline|RotateTimeline` :!via `PlayFromStart`)
        (:`Update`
          (bind _returnvalue_2 (`KismetMathLibrary.Lerp` _output_get _output_get_2 _lerp_alpha))
          (`Controller.SetControlRotation` _returnvalue (`KismetMathLibrary.MakeRotator` (.roll (`Controller.GetControlRotation` _returnvalue)) (.pitch (`Controller.GetControlRotation` _returnvalue)) _returnvalue_2))
          (`self.K2_SetActorRotation` (`KismetMathLibrary.MakeRotator` (.roll (`self.K2_GetActorRotation`)) (.pitch (`self.K2_GetActorRotation`)) _returnvalue_2))
          (if (== _lerp_alpha 1.0)
            (set `self.InputLock` false)
            (`TimelineComponent.Stop` (`self.RotateTimeline`))
            (bind _currentgamephase (`/Game/_MainProject/Blueprints/FunctionLibrary.CheckGamePhase` :!label _label_2))
            (switch `/Game/_MainProject/Blueprints/Enumerations/EnumGamePhase` _currentgamephase
              (:`NewEnumerator0`
                (goto _label :!via `Reset`))
              (:`NewEnumerator1`
                (bind (_targetfound _targetactor _isally) (`self.GetTargetFront`))
                (if (and _targetfound (not _isally))
                  (bind _asenemy_base (cast `/Game/_MainProject/Blueprints/Actors/EnemyBase` _targetactor))
                  (`/Game/_MainProject/Blueprints/Actors/EnemyBase.LoadCombatHUD` _asenemy_base)
                  (goto _label :!via `Reset`)
                  (else
                    (goto _label :!via `Reset`)))))))
        (:`Finished`
          (goto _label_2))))))

(event `self.ReceiveBeginPlay`
  (`|ExecutionSequence`
    (:`then_0`
      (bind _returnvalue (`|CreateWidget` "/Game/_MainProject/Blueprints/Widgets/HUD.HUD_C"))
      (`UserWidget.AddToViewport` _returnvalue 0)
      (set `PlayerController.bShowMouseCursor` true (`GameplayStatics.GetPlayerController` 0))
      (set `self.HUD` _returnvalue))
    (:`then_1`
      (bind _asrun_info_game_instance (cast `/Game/_MainProject/Blueprints/GameModes/RunInfo_GameInstance` (`GameplayStatics.GetGameInstance`)))
      (if (== (`/Game/_MainProject/Blueprints/GameModes/RunInfo_GameInstance.Floor` _asrun_info_game_instance) 1)
        (bind _as_dev_room_game_mode (cast `/Game/_MainProject/Blueprints/GameModes/_DevRoomGameMode` (`GameplayStatics.GetGameMode`)))
        (`/Game/_MainProject/Blueprints/GameModes/_DevRoomGameMode.GenerateStarterDice` _as_dev_room_game_mode)))
    (:`then_2`
      (set `PlayerController.bEnableMouseOverEvents` true (`GameplayStatics.GetPlayerController` 0)))
    (:`then_3`
      (bind _returnvalue_2 (`|CreateWidget` "/Game/_MainProject/Blueprints/Widgets/Combat/CombatHUD.CombatHUD_C"))
      (`UserWidget.AddToViewport` _returnvalue_2 0)
      (set `self.CombatHUD` _returnvalue_2))
    (:`then_4`
      (bind _as_dev_room_game_mode_2 (cast `/Game/_MainProject/Blueprints/GameModes/_DevRoomGameMode` (`GameplayStatics.GetGameMode`)))
      (`KismetArrayLibrary.Array_AddUnique` (`/Game/_MainProject/Blueprints/GameModes/_DevRoomGameMode.CharactersArray` _as_dev_room_game_mode_2) self))
    (:`then_5`
      (set `self.LevelRequirement` (`/Game/_MainProject/Blueprints/GameModes/_DevRoomGameMode.LevelRequirement` _as_dev_room_game_mode_2))
      (`self.RefreshLevel`))))

(event `InputAction|Interact`
  (params (Key :type "Key Structure"))
  (:`Pressed`
    (message `/Game/_MainProject/Blueprints/GameModes/Managers/ExplorationInterface.InteractWithActor` (`self.InteractibleTargetRef`))))

(event `InputAction|Inventory`
  (params (Key :type "Key Structure"))
  (bind _inventory (`/Game/_MainProject/Blueprints/Widgets/HUD.Inventory` (`self.HUD`)))
  (:`Pressed`
    (if (`Widget.IsVisible` _inventory)
      (`/Game/_MainProject/Blueprints/Widgets/Inventory/Inventory.CloseWidget` _inventory)
      (else
        (`Widget.SetVisibility` _inventory "SelfHitTestInvisible")
        (`/Game/_MainProject/Blueprints/Widgets/Inventory/Inventory.AddToCloseListenQueue` _inventory)))))

(event `InputAction|RotateLeft`
  (params (Key :type "Key Structure"))
  ;[1 1 1] Rotate Camera and Character
  (:`Pressed`
    (if (not (`self.InputLock`))
      (bind _currentgamephase (`/Game/_MainProject/Blueprints/FunctionLibrary.CheckGamePhase`))
      (switch `/Game/_MainProject/Blueprints/Enumerations/EnumGamePhase` _currentgamephase
        (:`NewEnumerator0`
          _)
        (:`NewEnumerator1`
          (`self.HideEnemyHUD`)))
      (`self.Rotate` -90.0))))

(event `InputAction|RotateRight`
  (params (Key :type "Key Structure"))
  ;[1 1 1] Rotate Camera and Character
  (:`Pressed`
    (if (not (`self.InputLock`))
      (bind _currentgamephase (`/Game/_MainProject/Blueprints/FunctionLibrary.CheckGamePhase`))
      (switch `/Game/_MainProject/Blueprints/Enumerations/EnumGamePhase` _currentgamephase
        (:`NewEnumerator0`
          _)
        (:`NewEnumerator1`
          (`self.HideEnemyHUD`)))
      (`self.Rotate` 90.0))))

(event `Movement`
  (params (Direction :type "Vector Structure"))
  (bind _returnvalue (`self.K2_GetActorLocation`))
  ;[1 1 1] Movement
  (bind _asmanagers_game_state (cast `/Game/_MainProject/Blueprints/GameModes/Managers/Managers_GameState` (`GameplayStatics.GetGameState`)))
  (if (not (`ActorComponent.IsActive` (`/Game/_MainProject/Blueprints/GameModes/Managers/Managers_GameState.CombatManager` _asmanagers_game_state)))
    (set `self.InputLock` true)
    (`/Engine/EditorBlueprintResources/StandardMacros.DoOnce` false :!label _label_3
      (:`Completed`
        (bind _output_get (set `self.StartLocation` _returnvalue))
        (bind _output_get_2 (set `self.EndLocation` (+ _returnvalue (* Direction 400.0))))
        (bind _outactors (`GameplayStatics.GetAllActorsWithTag` "Loot"))
        (bind (_outhit _returnvalue_2) (`KismetSystemLibrary.LineTraceSingle` _output_get _output_get_2 "TraceTypeQuery1" false _outactors "ForOneFrame")) ; Check for Collision
        (if _returnvalue_2
          (set `self.InputLock` false :!label _label_4)
          (`TimelineComponent.Stop` (`self.MovementTimeline`))
          (`self.ReduceMovesLeft` 1 :!label _label_5)
          (goto _label_3 :!via `Reset`)
          (else
            (bind (_direction _lerp_alpha) (`Timeline|MovementTimeline` :`NewTime` 1.0 :!via `PlayFromStart`)
              (:`Update`
                (`self.K2_SetActorLocation` (`KismetMathLibrary.VLerp` _output_get _output_get_2 _lerp_alpha))
                (if (== _lerp_alpha 1.0)
                  (goto _label_4)))
              (:`Finished`
                (goto _label_5)))))))))

(event `/Game/_MainProject/Blueprints/GameModes/Managers/ExplorationInterface.StartExplorationTurn`
  (set `self.InputLock` false))

(event `InputAction|MoveForward`
  (params (Key :type "Key Structure"))
  ;[1 1 1] Movement
  (:`Pressed`
    (if (not (`self.InputLock`))
      (`self.Movement` (`KismetMathLibrary.Normal` (* (select `bool` (`HeadMountedDisplayFunctionLibrary.IsHeadMountedDisplayEnabled`) :`false` (`self.GetActorForwardVector`) :`true` (`SceneComponent.GetForwardVector` (`self.FollowCamera`))) 1.0))))))

(event `PlayerEndOfExplorationTurn`
  (set `self.InputLock` true))

(event `InputAction|SkipTurn`
  (params (Key :type "Key Structure"))
  (:`Pressed`
    (bind _currentgamephase (`/Game/_MainProject/Blueprints/FunctionLibrary.CheckGamePhase`))
    (switch `/Game/_MainProject/Blueprints/Enumerations/EnumGamePhase` _currentgamephase
      (:`NewEnumerator0`
        (`self.EndExplorationTurn`))
      (:`NewEnumerator1`
        (`self.EndCombatTurn`)))))

(event `InputAction|MoveBackwards`
  (params (Key :type "Key Structure"))
  ;[1 1 1] Movement
  (:`Pressed`
    (if (not (`self.InputLock`))
      (`self.Movement` (`KismetMathLibrary.Normal` (* (select `bool` (`HeadMountedDisplayFunctionLibrary.IsHeadMountedDisplayEnabled`) :`false` (`self.GetActorForwardVector`) :`true` (`SceneComponent.GetForwardVector` (`self.FollowCamera`))) -1.0))))))

(event `InputAction|MoveRight`
  (params (Key :type "Key Structure"))
  ;[1 1 1] Movement
  (:`Pressed`
    (if (not (`self.InputLock`))
      (`self.Movement` (`KismetMathLibrary.Normal` (* (select `bool` (`HeadMountedDisplayFunctionLibrary.IsHeadMountedDisplayEnabled`) :`false` (`self.GetActorRightVector`) :`true` (`SceneComponent.GetRightVector` (`self.FollowCamera`))) 1.0))))))

(event `InputAction|MoveLeft`
  (params (Key :type "Key Structure"))
  ;[1 1 1] Movement
  (:`Pressed`
    (if (not (`self.InputLock`))
      (`self.Movement` (`KismetMathLibrary.Normal` (* (select `bool` (`HeadMountedDisplayFunctionLibrary.IsHeadMountedDisplayEnabled`) :`false` (`self.GetActorRightVector`) :`true` (`SceneComponent.GetRightVector` (`self.FollowCamera`))) -1.0))))))

(event `OpenCombatScreen`
  (bind _combathud (`self.CombatHUD`))
  (`/Game/_MainProject/Blueprints/Widgets/Combat/CombatHUD.ReConstruct` _combathud)
  (`Widget.SetVisibility` (`self.HUD`) "Hidden")
  (`Widget.SetVisibility` _combathud "SelfHitTestInvisible"))

(event `EndCombatPlayer`
  (`Widget.SetVisibility` (`self.CombatHUD`) "Hidden")
  (`/Game/_MainProject/Blueprints/Widgets/HUD.UpdateDiceSlots` (`self.HUD`))
  (`Widget.SetVisibility` (`self.HUD`) "SelfHitTestInvisible"))

(event `/Game/_MainProject/Blueprints/GameModes/Managers/CombatInterface.StartCombatTurn`
  (bind _combathud (`self.CombatHUD`))
  (`/Game/_MainProject/Blueprints/Widgets/Combat/CombatHUD.StartTurn` _combathud)
  (`Widget.SetVisibility` _combathud "SelfHitTestInvisible"))

(event `RefreshLevel`
  (bind (_playerexp _requiredexp _levelupinstances) (`/Game/_MainProject/Blueprints/DataTables/LevelRequirementCalculation.ValidateEXP` (`self.LevelRequirement`) (`self.CurrentLevel`) (`self.CurrentEXP`)))
  (`TextBlock.SetText` (`/Game/_MainProject/Blueprints/Widgets/HUD.ExpTextBLock` (`self.HUD`)) (`|FormatText` "Exp: {Current}/{NextLevel}" _playerexp _requiredexp))
  (`self.LevelUp` _levelupinstances))

(event `LevelUp`
  (params (Instances :type Integer))
  (for _ (range 1 (+ Instances 1))
    (`KismetSystemLibrary.PrintString` ">> LEVEL UP")))

(event `AddEXP`
  (params (EXP :type Integer))
  ;[1 1 1] DEBUG ONLY
  (set `self.CurrentEXP` (+ (`self.CurrentEXP`) EXP))
  (`self.RefreshLevel`))

(fn `GetTargetFront`
  (returns (TargetFound :type Boolean) (TargetActor :type "/Game/_MainProject/Blueprints/Actors/CombatCharacterBase Object Reference") (IsAlly :type Boolean))
  (bind _returnvalue (`self.K2_GetActorLocation` self))
  ;[1 1 1] Find target in Front
  (bind _outactors (`GameplayStatics.GetAllActorsWithTag` "Loot"))
  (bind (_outhit _returnvalue_2) (`KismetSystemLibrary.LineTraceSingle` _returnvalue (+ _returnvalue (* (`KismetMathLibrary.GetForwardVector` (`SceneComponent.K2_GetComponentRotation` (`self.CapsuleComponent`))) 400.0)) "TraceTypeQuery1" false _outactors "ForOneFrame"))
  (if _returnvalue_2
    (bind (_bblockinghit _binitialoverlap _time _distance _location _impactpoint _normal _impactnormal _physmat _hitactor) (`GameplayStatics.BreakHitResult` _outhit))
    (bind _ascombat_character_base (cast `/Game/_MainProject/Blueprints/Actors/CombatCharacterBase` _hitactor)
      (:`then`
        (bind _asmanagers_game_state (cast `/Game/_MainProject/Blueprints/GameModes/Managers/Managers_GameState` (`GameplayStatics.GetGameState`)))
        (bind _returnvalue_3 (`KismetArrayLibrary.Array_Contains` (`/Game/_MainProject/Blueprints/GameModes/Managers/CombatManager.CombatantsArray` (`/Game/_MainProject/Blueprints/GameModes/Managers/Managers_GameState.CombatManager` _asmanagers_game_state)) _ascombat_character_base))
        (bind _returnvalue_4 (not _returnvalue_3))
        (`KismetSystemLibrary.PrintString` "///Get Target Front >> Hit target does not take part in current combat" _returnvalue_4 _returnvalue_4)
        (return _returnvalue_3 _ascombat_character_base (not (`self.ActorHasTag` _hitactor "Hostile"))))
      (:`CastFailed`
        (`KismetSystemLibrary.PrintString` "///Get Target Front >> Hit target is not a Combat Based Character")))
    (else
      (`KismetSystemLibrary.PrintString` "///Get Target Front >> No target found")))
  (return false null false))

(fn `GetTotalDicesInSlot`
  (params (StatAssignment :type "/Game/_MainProject/Blueprints/Enumerations/Dice/EnumStatAssignment Enum" :default "NewEnumerator0"))
  (returns (ReturnDiceCount :type Integer) (DiceArray :type "Array of /Game/_MainProject/Blueprints/Widgets/Dice/Dice Object Reference"))
  (locals (DiceCount :type Integer) (DiceInSlotArray :type "Array of /Game/_MainProject/Blueprints/Widgets/Dice/Dice Object Reference"))
  (for _array_element (`self.DiceArray`)
    (if (`|EnumEquality` (`/Game/_MainProject/Blueprints/Widgets/Dice/Dice.StatAssignment` _array_element) StatAssignment)
      (`/Engine/EditorBlueprintResources/StandardMacros.IncrementInt` (`local.DiceCount`)
        (:`  `
          (`KismetArrayLibrary.Array_Add` (`local.DiceInSlotArray`) _array_element)))))
  (return (`local.DiceCount`) (`local.DiceInSlotArray`)))

(fn `UserConstructionScript`)