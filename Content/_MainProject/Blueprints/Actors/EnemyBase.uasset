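; Base enemy Blueprint that lets the player start combat with it and owns its combat HUD.
; Cursor hover shows an "Engage Combat" prompt and sets the player's interaction target if the player is near, facing it and out of combat.
; Interacting repeats the range and yaw check, then calls BeginCombat on the GameState.
; The HUD loads on demand, hides on CombatManager or player-rotation events, and is removed with the prompt on destruction.
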(event `self.ReceiveBeginPlay`
  (`parent.ReceiveBeginPlay`)
  (`|ExecutionSequence`
    (:`then_0`
      (bind _returnvalue (`|CreateWidget` "/Game/_MainProject/Blueprints/Widgets/InteractPrompt.InteractPrompt_C" null "Engage Combat" "F"))
      (bind _output_get (set `self.InteractPromptRef` _returnvalue))
      (`UserWidget.AddToViewport` _output_get 0))
    (:`then_1`
      (if (not (`KismetSystemLibrary.IsValid` (`self.CombatHUD`)))
        (bind _returnvalue_2 (`|CreateWidget` "/Game/_MainProject/Blueprints/Widgets/Combat/EnemyCombatHUD.EnemyCombatHUD_C" null self))
        (set `self.CombatHUD` _returnvalue_2)))
    (:`then_2`
      (bind _asmanagers_game_state (cast `/Game/_MainProject/Blueprints/GameModes/Managers/Managers_GameState` (`GameplayStatics.GetGameState`)))
      (add `/Game/_MainProject/Blueprints/GameModes/Managers/CombatManager.HideEnemyHUD` (`/Game/_MainProject/Blueprints/GameModes/Managers/Managers_GameState.CombatManager` _asmanagers_game_state) (delegate `HideCombatHUD`))
      (bind _asbp_player (cast `/Game/_MainProject/Blueprints/Actors/BP_Player` (`GameplayStatics.GetPlayerCharacter` 0)))
      (add `/Game/_MainProject/Blueprints/Actors/BP_Player.HideEnemyHUD` _asbp_player (delegate `HideCombatHUD-PlayerStartRotate`)))))

(event `HideCombatHUD`
  (`Widget.SetVisibility` (`self.CombatHUD`) "Collapsed" :!label _label))

(event `HideCombatHUD-PlayerStartRotate`
  (goto _label))

(event `self.Mesh.OnBeginCursorOver`
  (params (TouchedComponent :type "PrimitiveComponent Object Reference"))
  (bind _returnvalue (`GameplayStatics.GetPlayerCharacter` 0))
  (bind _returnvalue_2 (`KismetMathLibrary.Round` (`KismetMathLibrary.Abs` (- (.yaw (`self.GetControlRotation` _returnvalue)) (.yaw (`KismetMathLibrary.FindLookAtRotation` (`self.K2_GetActorLocation` _returnvalue) (`self.K2_GetActorLocation` self)))))))
  (if (and (<= (`KismetMathLibrary.Abs` (- (.x (`SceneComponent.K2_GetComponentLocation` (`self.Mesh`))) (.x (`SceneComponent.K2_GetComponentLocation` (`Character.Mesh` (`GameplayStatics.GetPlayerCharacter` 0)))))) 600.0) (<= (`KismetMathLibrary.Abs` (- (.y (`SceneComponent.K2_GetComponentLocation` (`self.Mesh`))) (.y (`SceneComponent.K2_GetComponentLocation` (`Character.Mesh` (`GameplayStatics.GetPlayerCharacter` 0)))))) 600.0) (or (== _returnvalue_2 0) (== _returnvalue_2 360)))
    (bind _asmanagers_game_state (cast `/Game/_MainProject/Blueprints/GameModes/Managers/Managers_GameState` (`GameplayStatics.GetGameState`)))
    (if (not (`ActorComponent.IsActive` (`/Game/_MainProject/Blueprints/GameModes/Managers/Managers_GameState.CombatManager` _asmanagers_game_state)))
      (`Widget.SetVisibility` (`self.InteractPromptRef`) "HitTestInvisible")
      (bind _asbp_player (cast `/Game/_MainProject/Blueprints/Actors/BP_Player` (`GameplayStatics.GetPlayerCharacter` 0)))
      (set `/Game/_MainProject/Blueprints/Actors/BP_Player.InteractibleTargetRef` self _asbp_player))))

(event `self.Mesh.OnEndCursorOver`
  (params (TouchedComponent :type "PrimitiveComponent Object Reference"))
  (`Widget.SetVisibility` (`self.InteractPromptRef`) "Collapsed")
  (bind _asbp_player (cast `/Game/_MainProject/Blueprints/Actors/BP_Player` (`GameplayStatics.GetPlayerCharacter` 0)))
  (set `/Game/_MainProject/Blueprints/Actors/BP_Player.InteractibleTargetRef` (`/Game/_MainProject/Blueprints/Actors/BP_Player.InteractibleTargetRef_RESET` _asbp_player) _asbp_player))

(event `/Game/_MainProject/Blueprints/GameModes/Managers/ExplorationInterface.InteractWithActor`
  (bind _returnvalue (`GameplayStatics.GetPlayerCharacter` 0))
  (bind _returnvalue_2 (`KismetMathLibrary.Round` (`KismetMathLibrary.Abs` (- (.yaw (`self.GetControlRotation` _returnvalue)) (.yaw (`KismetMathLibrary.FindLookAtRotation` (`self.K2_GetActorLocation` _returnvalue) (`self.K2_GetActorLocation` self)))))))
  (if (and (<= (`KismetMathLibrary.Abs` (- (.x (`SceneComponent.K2_GetComponentLocation` (`self.Mesh`))) (.x (`SceneComponent.K2_GetComponentLocation` (`Character.Mesh` (`GameplayStatics.GetPlayerCharacter` 0)))))) 600.0) (<= (`KismetMathLibrary.Abs` (- (.y (`SceneComponent.K2_GetComponentLocation` (`self.Mesh`))) (.y (`SceneComponent.K2_GetComponentLocation` (`Character.Mesh` (`GameplayStatics.GetPlayerCharacter` 0)))))) 600.0) (or (== _returnvalue_2 0) (== _returnvalue_2 360)))
    (bind _asmanagers_game_state (cast `/Game/_MainProject/Blueprints/GameModes/Managers/Managers_GameState` (`GameplayStatics.GetGameState`)))
    (bind _ascombat_character_base (cast `/Game/_MainProject/Blueprints/Actors/CombatCharacterBase` (`GameplayStatics.GetPlayerCharacter` 0)))
    (`/Game/_MainProject/Blueprints/GameModes/Managers/Managers_GameState.BeginCombat` _asmanagers_game_state _ascombat_character_base self)))

(event `LoadCombatHUD`
  (bind _combathud (`self.CombatHUD`))
  (if (not (`Widget.IsInViewport` _combathud))
    (`UserWidget.AddToViewport` _combathud 1)
    (else
      (`Widget.SetVisibility` _combathud "SelfHitTestInvisible"))))

(event `self.ReceiveDestroyed`
  (`|ExecutionSequence`
    (:`then_0`
      (`Widget.RemoveFromParent` (`self.InteractPromptRef`)))
    (:`then_1`
      (`Widget.RemoveFromParent` (`self.CombatHUD`)))))

(fn `UserConstructionScript`)