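; Shared function library for a dice-based game, covering equipment and dice creation, dice queries, UI sizing, error printing and game-phase lookup.
; Equipment helpers map rarity to DataTables (only Starter is assigned) and build widgets from rows.
; Random picks and weighted dice size/type generation draw on the GameInstance's seed stream; the d12 and d20 branches never reach widget creation.
; Dice helpers filter by slot or type, find highest values, reroll and re-parent.
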(fn `CheckGamePhase`
  (returns (CurrentGamePhase :type "/Game/_MainProject/Blueprints/Enumerations/EnumGamePhase Enum"))
  (bind _asmanagers_game_state (cast `/Game/_MainProject/Blueprints/GameModes/Managers/Managers_GameState` (`GameplayStatics.GetGameState` null)))
  (if (`ActorComponent.IsActive` (`/Game/_MainProject/Blueprints/GameModes/Managers/Managers_GameState.CombatManager` _asmanagers_game_state))
    (return "NewEnumerator1")
    (else
      (return (`/Game/_MainProject/Blueprints/GameModes/Managers/ExplorationManager.GamePhase` (`/Game/_MainProject/Blueprints/GameModes/Managers/Managers_GameState.ExplorationManager` _asmanagers_game_state))))))

(fn `DebugErrorPrint`
  (params (WorldContextObject :type "Object Object Reference") (SourceBlueprint :type String) (Cause :type Text))
  (`KismetSystemLibrary.PrintString` WorldContextObject (`KismetTextLibrary.Conv_TextToString` (`|FormatText` "/// \nERROR \nSource: {SourceBlueprint} \nReason: {Cause} \n///" SourceBlueprint Cause)) true true (struct :`R` 1.0 :`A` 1.0) 10.0))

(fn `GenerateRandomDice`
  (params (WorldContextObject :type "Object Object Reference"))
  (returns (`Created Dice` :type "/Game/_MainProject/Blueprints/Widgets/Dice/Dice Object Reference"))
  (locals (TmpDiceSize :type Integer) (TmpEnumDice :type "/Game/_MainProject/Blueprints/Enumerations/Dice/EnumDice Enum") (TmpGold :type Integer))
  (bind _asrun_info_game_instance (cast `/Game/_MainProject/Blueprints/GameModes/RunInfo_GameInstance` (`GameplayStatics.GetGameInstance` WorldContextObject)))
  (bind _seed (`/Game/_MainProject/Blueprints/GameModes/RunInfo_GameInstance.Seed` _asrun_info_game_instance))
  ;[1 1 1] Generate Dice Size
  (switch `int` (`KismetMathLibrary.RandomIntegerFromStream` 20 _seed)
    (:`0`
      (switch `int` (`KismetMathLibrary.RandomIntegerFromStream` 2 _seed) :!label _label
        (:`0`
          (set `local.TmpDiceSize` 4))
        (:`1`
          (set `local.TmpDiceSize` 6)))
      ;[1 1 1] Generate Dice Type
      (switch `int` (`KismetMathLibrary.RandomIntegerFromStream` 20 _seed) :!label _label_2
        (:`0`
          (set `local.TmpEnumDice` "NewEnumerator0" :!label _label_3))
        (:`1`
          (goto _label_3))
        (:`2`
          (goto _label_3))
        (:`3`
          (goto _label_3))
        (:`4`
          (goto _label_3))
        (:`5`
          (goto _label_3))
        (:`6`
          (goto _label_3))
        (:`7`
          (goto _label_3))
        (:`8`
          (goto _label_3))
        (:`9`
          (goto _label_3))
        (:`10`
          (goto _label_3))
        (:`11`
          (set `local.TmpEnumDice` (cast `/Game/_MainProject/Blueprints/Enumerations/Dice/EnumDice` (`KismetMathLibrary.Conv_IntToByte` (+ (`KismetMathLibrary.RandomIntegerFromStream` 5 _seed) 1))) :!label _label_4))
        (:`12`
          (goto _label_4))
        (:`13`
          (goto _label_4))
        (:`14`
          (goto _label_4))
        (:`15`
          (goto _label_4))
        (:`16`
          (goto _label_4))
        (:`17`
          (goto _label_4))
        (:`18`
          (set `local.TmpEnumDice` "NewEnumerator6"))
        (:`19`
          (set `local.TmpEnumDice` "NewEnumerator7")
          (set `local.TmpGold` (`KismetMathLibrary.RandomIntegerFromStream` (`KismetMathLibrary.FTrunc` (* (`local.TmpDiceSize`) 0.25)) _seed))))
      ;[1 1 1] Create Dice
      (bind _returnvalue (`|CreateWidget` :`Class` "/Game/_MainProject/Blueprints/Widgets/Dice/Dice.Dice_C" :`DiceSize` (`local.TmpDiceSize`) :`DiceType` (`local.TmpEnumDice`) :`Gold` (`local.TmpGold`) :`Owner` null))
      (return _returnvalue))
    (:`1`
      (goto _label))
    (:`2`
      (goto _label))
    (:`3`
      (goto _label))
    (:`4`
      (goto _label))
    (:`5`
      (goto _label))
    (:`6`
      (goto _label))
    (:`7`
      (goto _label))
    (:`8`
      (goto _label))
    (:`9`
      (goto _label))
    (:`10`
      (goto _label))
    (:`11`
      (switch `int` (`KismetMathLibrary.RandomIntegerFromStream` 2 _seed) :!label _label_5
        (:`0`
          (set `local.TmpDiceSize` 8)
          (goto _label_2))
        (:`1`
          (set `local.TmpDiceSize` 10)
          (goto _label_2))))
    (:`12`
      (goto _label_5))
    (:`13`
      (goto _label_5))
    (:`14`
      (goto _label_5))
    (:`15`
      (goto _label_5))
    (:`16`
      (goto _label_5))
    (:`17`
      (goto _label_5))
    (:`18`
      (set `local.TmpDiceSize` 12))
    (:`19`
      (set `local.TmpDiceSize` 20))))

(fn `GetAllEquipmentFromNames`
  (params (`Out Row Names` :type "Array of Name") (`Selected DataTable` :type "DataTable Object Reference"))
  (returns (EquipmentArray :type "Array of /Game/_MainProject/Blueprints/Widgets/Inventory/Equipment/EquipmentWidget Object Reference"))
  (locals (TmpEquipmentArray :type "Array of /Game/_MainProject/Blueprints/Widgets/Inventory/Equipment/EquipmentWidget Object Reference") (CreatedEquipment :type "/Game/_MainProject/Blueprints/Widgets/Inventory/Equipment/EquipmentWidget Object Reference"))
  (for _array_element `Out Row Names`
    (bind _returnvalue (`|GetDataTableRow` `Selected DataTable` _array_element)
      (:`then`
        (bind _returnvalue_2 (`|CreateWidget` "/Game/_MainProject/Blueprints/Widgets/Inventory/Equipment/EquipmentWidget.EquipmentWidget_C" null _returnvalue 20.0 null))
        (`KismetArrayLibrary.Array_Add` (`local.TmpEquipmentArray`) _returnvalue_2))
      (:`RowNotFound`
        (`KismetSystemLibrary.PrintString` null (`KismetTextLibrary.Conv_TextToString` (`|FormatText` "ERROR: Failed to find Row Name {Row Name} in {DataTable} DataTable" _array_element (`KismetSystemLibrary.GetDisplayName` `Selected DataTable`)))))))
  (return (`local.TmpEquipmentArray`)))

(fn `GetAllEquipmentFromRarity`
  (params (Rarity :type "/Game/_MainProject/Blueprints/Enumerations/EnumRarity Enum" :default "NewEnumerator0"))
  (returns (Equipment :type "Array of /Game/_MainProject/Blueprints/Widgets/Inventory/Equipment/EquipmentWidget Object Reference"))
  (bind (_out_row_names _selected_datatable) (`self.GetEquipmentListQuery` Rarity (`local.__WorldContext`)))
  (bind _equipmentarray (`self.GetAllEquipmentFromNames` _out_row_names _selected_datatable (`local.__WorldContext`)))
  (return _equipmentarray))

(fn `GetDicesInSlot`
  (params (InputDiceArray :type "Array of /Game/_MainProject/Blueprints/Widgets/Dice/Dice Object Reference") (StatAssignment :type "/Game/_MainProject/Blueprints/Enumerations/Dice/EnumStatAssignment Enum" :default "NewEnumerator0"))
  (returns (ReturnDiceCount :type Integer) (FilteredDiceArray :type "Array of /Game/_MainProject/Blueprints/Widgets/Dice/Dice Object Reference"))
  (locals (DiceCount :type Integer) (DiceInSlotArray :type "Array of /Game/_MainProject/Blueprints/Widgets/Dice/Dice Object Reference"))
  (for _array_element InputDiceArray
    (if (`|EnumEquality` (`/Game/_MainProject/Blueprints/Widgets/Dice/Dice.StatAssignment` _array_element) StatAssignment)
      (`/Engine/EditorBlueprintResources/StandardMacros.IncrementInt` (`local.DiceCount`)
        (:`  `
          (`KismetArrayLibrary.Array_Add` (`local.DiceInSlotArray`) _array_element)))))
  (return (`local.DiceCount`) (`local.DiceInSlotArray`)))

(fn `GetDicesOfType`
  (params (InputDiceArray :type "Array of /Game/_MainProject/Blueprints/Widgets/Dice/Dice Object Reference") (DiceType :type "/Game/_MainProject/Blueprints/Enumerations/Dice/EnumDice Enum" :default "NewEnumerator0"))
  (returns (ReturnDiceCount :type Integer) (FilteredDiceArray :type "Array of /Game/_MainProject/Blueprints/Widgets/Dice/Dice Object Reference"))
  (locals (DiceCount :type Integer) (DiceOfTypeArray :type "Array of /Game/_MainProject/Blueprints/Widgets/Dice/Dice Object Reference"))
  (for _array_element InputDiceArray
    (if (`|EnumEquality` (`/Game/_MainProject/Blueprints/Widgets/Dice/Dice.DiceType` _array_element) DiceType)
      (`/Engine/EditorBlueprintResources/StandardMacros.IncrementInt` (`local.DiceCount`)
        (:`  `
          (`KismetArrayLibrary.Array_Add` (`local.DiceOfTypeArray`) _array_element)))))
  (return (`local.DiceCount`) (`local.DiceOfTypeArray`)))

(fn `GetEquipmentListQuery`
  (params (Rarity :type "/Game/_MainProject/Blueprints/Enumerations/EnumRarity Enum" :default "NewEnumerator0"))
  (returns (`Out Row Names` :type "Array of Name") (`Selected DataTable` :type "DataTable Object Reference"))
  (locals (TmpDataTable :type "DataTable Object Reference"))
  (switch `/Game/_MainProject/Blueprints/Enumerations/EnumRarity` Rarity
    (:`NewEnumerator0`
      (set `local.TmpDataTable` null))
    (:`NewEnumerator1`
      (set `local.TmpDataTable` null))
    (:`NewEnumerator2`
      (set `local.TmpDataTable` null))
    (:`NewEnumerator3`
      (set `local.TmpDataTable` null))
    (:`NewEnumerator4`
      (set `local.TmpDataTable` "/Game/_MainProject/Blueprints/DataTables/StarterEquipmentDataTable.StarterEquipmentDataTable")))
  (bind _outrownames (`DataTableFunctionLibrary.GetDataTableRowNames` (`local.TmpDataTable`)))
  (return _outrownames (`local.TmpDataTable`)))

(fn `GetHighestValueAmongDiceArray`
  (params (InputDiceArray :type "Array of /Game/_MainProject/Blueprints/Widgets/Dice/Dice Object Reference"))
  (returns (HighestValueFound :type Integer) (DiceWithHighestValue :type "/Game/_MainProject/Blueprints/Widgets/Dice/Dice Object Reference"))
  (locals (HighestValue :type Integer) (DiceReference :type "/Game/_MainProject/Blueprints/Widgets/Dice/Dice Object Reference"))
  (for (_array_element _array_index) InputDiceArray
    (if (== _array_index 0)
      (bind _highestvalue (`/Game/_MainProject/Blueprints/Widgets/Dice/Dice.Get Highest Value` _array_element))
      (set `local.HighestValue` _highestvalue)
      (set `local.DiceReference` _array_element)
      (else
        (bind _highestvalue_2 (`/Game/_MainProject/Blueprints/Widgets/Dice/Dice.Get Highest Value` _array_element))
        (if (> _highestvalue_2 (`local.HighestValue`))
          (set `local.HighestValue` _highestvalue_2)
          (set `local.DiceReference` _array_element)))))
  (return (`local.HighestValue`) (`local.DiceReference`)))

(fn `GetHighestValueAmongSlot`
  (params (InputDiceArray :type "Array of /Game/_MainProject/Blueprints/Widgets/Dice/Dice Object Reference") (StatAssignment :type "/Game/_MainProject/Blueprints/Enumerations/Dice/EnumStatAssignment Enum" :default "NewEnumerator0"))
  (returns (HighestValueInSlot :type Integer) (DiceWithHighestValueInSlot :type "/Game/_MainProject/Blueprints/Widgets/Dice/Dice Object Reference"))
  (locals (HighestValue :type Integer) (DiceReference :type "/Game/_MainProject/Blueprints/Widgets/Dice/Dice Object Reference"))
  (bind (_returndicecount _filtereddicearray) (`self.GetDicesInSlot` InputDiceArray StatAssignment (`local.__WorldContext`)))
  (for (_array_element _array_index) _filtereddicearray
    (if (== _array_index 0)
      (bind _highestvalue (`/Game/_MainProject/Blueprints/Widgets/Dice/Dice.Get Highest Value` _array_element))
      (set `local.HighestValue` _highestvalue)
      (set `local.DiceReference` _array_element)
      (else
        (bind _highestvalue_2 (`/Game/_MainProject/Blueprints/Widgets/Dice/Dice.Get Highest Value` _array_element))
        (if (> _highestvalue_2 (`local.HighestValue`))
          (set `local.HighestValue` _highestvalue_2)
          (set `local.DiceReference` _array_element)))))
  (return (`local.HighestValue`) (`local.DiceReference`)))

(fn `GetRandomEquipmentFromNames`
  (params (`Out Row Names` :type "Array of Name") (`Selected DataTable` :type "DataTable Object Reference"))
  (returns (Equipment :type "/Game/_MainProject/Blueprints/Widgets/Inventory/Equipment/InventorySlotEquipmentWidget Object Reference"))
  (locals (CreatedEquipment :type "/Game/_MainProject/Blueprints/Widgets/Inventory/Equipment/EquipmentWidget Object Reference"))
  (bind _asrun_info_game_instance (cast `/Game/_MainProject/Blueprints/GameModes/RunInfo_GameInstance` (`GameplayStatics.GetGameInstance` (`local.__WorldContext`)))
    (:`then`
      (bind _output (`|GetArrayItem` `Out Row Names` (`KismetMathLibrary.RandomIntegerFromStream` (`KismetArrayLibrary.Array_Length` `Out Row Names`) (`/Game/_MainProject/Blueprints/GameModes/RunInfo_GameInstance.Seed` _asrun_info_game_instance))))
      (bind _returnvalue (`|GetDataTableRow` `Selected DataTable` _output)
        (:`then`
          (bind _returnvalue_2 (`|CreateWidget` "/Game/_MainProject/Blueprints/Widgets/Inventory/Equipment/EquipmentWidget.EquipmentWidget_C" null _returnvalue 20.0 null))
          (set `local.CreatedEquipment` _returnvalue_2)
          (bind _returnvalue_3 (`|CreateWidget` "/Game/_MainProject/Blueprints/Widgets/Inventory/Equipment/InventorySlotEquipmentWidget.InventorySlotEquipmentWidget_C" null null (`local.CreatedEquipment`)))
          (return _returnvalue_3))
        (:`RowNotFound`
          (`KismetSystemLibrary.PrintString` null (`KismetTextLibrary.Conv_TextToString` (`|FormatText` "ERROR: Failed to find Row Name {Row Name} in {DataTable} DataTable" _output (`KismetSystemLibrary.GetDisplayName` `Selected DataTable`)))))))
    (:`CastFailed`
      (`KismetSystemLibrary.PrintString` (`local.__WorldContext`) (`KismetTextLibrary.Conv_TextToString` (`|FormatText` "ERROR: Failed to cast to GameInstance"))))))

(fn `GetRandomEquipmentFromRarity`
  (params (Rarity :type "/Game/_MainProject/Blueprints/Enumerations/EnumRarity Enum" :default "NewEnumerator0"))
  (returns (Equipment :type "/Game/_MainProject/Blueprints/Widgets/Inventory/Equipment/InventorySlotEquipmentWidget Object Reference"))
  (bind (_out_row_names _selected_datatable) (`self.GetEquipmentListQuery` Rarity))
  (bind _equipment (`self.GetRandomEquipmentFromNames` _out_row_names _selected_datatable (`local.__WorldContext`)))
  (return _equipment))

(fn `RerollAllDice`
  (params (DiceArray :type "Array of /Game/_MainProject/Blueprints/Widgets/Dice/Dice Object Reference"))
  (for _array_element DiceArray
    (bind _statassignment (`/Game/_MainProject/Blueprints/Widgets/Dice/Dice.StatAssignment` _array_element))
    (if (and (`|EnumInequality` _statassignment "NewEnumerator1") (`|EnumInequality` _statassignment "NewEnumerator5") (not (`/Game/_MainProject/Blueprints/Widgets/Dice/Dice.UsedThisTurn` _array_element)))
      (`/Game/_MainProject/Blueprints/Widgets/Dice/Dice.RollRandom` _array_element))))

(fn `ResetDicePosition`
  (params (InputDiceArray :type "Array of /Game/_MainProject/Blueprints/Widgets/Dice/Dice Object Reference (by ref)") (WrapBoxArray :type "Array of WrapBox Object Reference (by ref)"))
  (for (_array_element _array_index) WrapBoxArray
    (bind (_returndicecount _filtereddicearray) (`self.GetDicesInSlot` InputDiceArray (`|GetArrayItem` (`|MakeArray` "NewEnumerator2" "NewEnumerator3" "NewEnumerator4" "NewEnumerator6" :!type "/Game/_MainProject/Blueprints/Enumerations/Dice/EnumStatAssignment Enum") _array_index) (`local.__WorldContext`)))
    (for _array_element_2 _filtereddicearray
      (if (not (`/Game/_MainProject/Blueprints/Widgets/Dice/Dice.UsedThisTurn` _array_element_2))
        (if (not (`PanelWidget.HasChild` _array_element _array_element_2))
          (`PanelWidget.AddChild` _array_element _array_element_2))
        (`/Game/_MainProject/Blueprints/Widgets/Dice/Dice.RollRandom` _array_element_2)))))

(fn `SetPositionOnCanvasPanel`
  (params (CanvasPanelSlot :type "CanvasPanelSlot Object Reference") (ScreenOffset :type "Float (double-precision)") (`X Scale` :type "Float (double-precision)" :default 1.0) (`Y Scale` :type "Float (double-precision)" :default 1.0))
  (bind (_x _y) (`KismetMathLibrary.BreakVector2D` (`CanvasPanelSlot.GetSize` CanvasPanelSlot)))
  (`CanvasPanelSlot.SetPosition` CanvasPanelSlot (`KismetMathLibrary.MakeVector2D` (* (+ _x ScreenOffset) `X Scale`) (* (+ _y ScreenOffset) `Y Scale`))))

(fn `SetSizeBoxOverrideToViewport`
  (params (`Size Box Reference` :type "SizeBox Object Reference") (`WidthOverride?` :type Boolean) (`Width%` :type "Float (double-precision)") (`HeightOverride?` :type Boolean) (`Height%` :type "Float (double-precision)") (WorldContextObject :type "Object Object Reference"))
  (bind (_x _y) (`KismetMathLibrary.BreakVector2D` (`WidgetLayoutLibrary.GetViewportSize` WorldContextObject)))
  (`|ExecutionSequence`
    (:`then_0`
      (if `WidthOverride?`
        (`SizeBox.SetWidthOverride` `Size Box Reference` (* `Width%` _x))))
    (:`then_1`
      (if `HeightOverride?`
        (`SizeBox.SetHeightOverride` `Size Box Reference` (* `Height%` _y))))))