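; Developer room game mode that starts a test run with a random seed, floor -1 and a debug movement die.
; Custom events open the dice spawn widget, remove dice widgets, spawn actors at a fixed spot and fill inventory with all equipment of one rarity.
; Starter dice generation draws from the seeded stream: four d4/d6 with at least one d6 and weighted types, plus a d20 with random gold.
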(event `self.ReceiveBeginPlay`
  (`|ExecutionSequence`
    (:`then_0`
      (bind _asrun_info_game_instance (cast `/Game/_MainProject/Blueprints/RunInfo_GameInstance` (`GameplayStatics.GetGameInstance`)))
      (set `/Game/_MainProject/Blueprints/RunInfo_GameInstance.Seed` (`KismetMathLibrary.MakeRandomStream` (`KismetMathLibrary.RandomInteger` 2147483647)) _asrun_info_game_instance)
      (set `/Game/_MainProject/Blueprints/RunInfo_GameInstance.Floor` -1 _asrun_info_game_instance))
    (:`then_1`
      (bind _returnvalue (`|CreateWidget` "/Game/_MainProject/Blueprints/Widgets/Debug/DebugMovementDice.DebugMovementDice_C"))
      (bind _ascombat_character_base (cast `/Game/_MainProject/Blueprints/Actors/CombatCharacterBase` (`GameplayStatics.GetPlayerCharacter` 0)))
      (`KismetArrayLibrary.Array_Add` (`/Game/_MainProject/Blueprints/Actors/CombatCharacterBase.DiceArray` _ascombat_character_base) _returnvalue))))

(event `CreateDice`
  (bind _foundwidgets (`WidgetBlueprintLibrary.GetAllWidgetsOfClass` "/Game/_MainProject/Blueprints/Widgets/Debug/DiceSpawnWidget.DiceSpawnWidget_C"))
  (if (== (`KismetArrayLibrary.Array_Length` _foundwidgets) 0)
    (bind _returnvalue (`|CreateWidget` "/Game/_MainProject/Blueprints/Widgets/Debug/DiceSpawnWidget.DiceSpawnWidget_C"))
    (`UserWidget.AddToViewport` _returnvalue 0)))

(event `RemoveAllDice`
  (bind _foundwidgets (`WidgetBlueprintLibrary.GetAllWidgetsOfClass` "/Game/_MainProject/Blueprints/Widgets/Dice/Dice.Dice_C" false))
  (for _array_element _foundwidgets
    (`Widget.RemoveFromParent` _array_element)))

(event `GenerateStarterDice`
  (bind _asrun_info_game_instance (cast `/Game/_MainProject/Blueprints/RunInfo_GameInstance` (`GameplayStatics.GetGameInstance`))
    (:`then`
      (for _index (range 4)
        (if (< _index 3)
          (bind _seed (`/Game/_MainProject/Blueprints/RunInfo_GameInstance.Seed` _asrun_info_game_instance))
          (switch `int` (`KismetMathLibrary.RandomIntegerFromStream` 2 _seed) :!label _label
            (:`0`
              (set `self.TmpInt` 4))
            (:`1`
              (set `self.TmpInt` 6)
              (set `self.TmpBool` true)))
          (elif (`self.TmpBool`)
            (goto _label)
            (else
              (set `self.TmpInt` 6))))
        (switch `int` (`KismetMathLibrary.RandomIntegerFromStream` 20 _seed)
          (:`0`
            (set `self.TmpInt_0` "NewEnumerator0" :!label _label_2))
          (:`1`
            (goto _label_2))
          (:`2`
            (goto _label_2))
          (:`3`
            (goto _label_2))
          (:`4`
            (goto _label_2))
          (:`5`
            (goto _label_2))
          (:`6`
            (goto _label_2))
          (:`7`
            (goto _label_2))
          (:`8`
            (goto _label_2))
          (:`9`
            (goto _label_2))
          (:`10`
            (goto _label_2))
          (:`11`
            (set `self.TmpInt_0` (cast `/Game/_MainProject/Blueprints/Enumerations/Dice/EnumDice` (`KismetMathLibrary.Conv_IntToByte` (+ (`KismetMathLibrary.RandomIntegerFromStream` 5 (`/Game/_MainProject/Blueprints/RunInfo_GameInstance.Seed` _asrun_info_game_instance)) 1))) :!label _label_3))
          (:`12`
            (goto _label_3))
          (:`13`
            (goto _label_3))
          (:`14`
            (goto _label_3))
          (:`15`
            (goto _label_3))
          (:`16`
            (goto _label_3))
          (:`17`
            (goto _label_3))
          (:`18`
            (set `self.TmpInt_0` "NewEnumerator6" :!label _label_4))
          (:`19`
            (goto _label_4)))
        (bind _returnvalue (`|CreateWidget` :`Class` "/Game/_MainProject/Blueprints/Widgets/Dice/Dice.Dice_C" :`DiceSize` (`self.TmpInt`) :`DiceType` (`self.TmpInt_0`) :`Gold` 0))
        (bind _asbp_player (cast `/Game/_MainProject/Blueprints/Actors/BP_Player` (`GameplayStatics.GetPlayerCharacter` 0)))
        (`KismetArrayLibrary.Array_Add` (`/Game/_MainProject/Blueprints/Actors/BP_Player.DiceArray` _asbp_player) _returnvalue))
      (bind _returnvalue_2 (`|CreateWidget` :`Class` "/Game/_MainProject/Blueprints/Widgets/Dice/Dice.Dice_C" :`DiceSize` 20 :`DiceType` "NewEnumerator7" :`Gold` (`KismetMathLibrary.RandomIntegerInRangeFromStream` 1 6 _seed)))
      (bind _asbp_player_2 (cast `/Game/_MainProject/Blueprints/Actors/BP_Player` (`GameplayStatics.GetPlayerCharacter` 0)))
      (`KismetArrayLibrary.Array_Add` (`/Game/_MainProject/Blueprints/Actors/BP_Player.DiceArray` _asbp_player_2) _returnvalue_2)
      (`/Game/_MainProject/Blueprints/Widgets/HUD.UpdateDiceSlots` (`/Game/_MainProject/Blueprints/Actors/BP_Player.HUD` _asbp_player_2)))
    (:`CastFailed`
      (`KismetSystemLibrary.PrintString` "Failed to load RunInfo_GameInstance"))))

(event `SpawnInteractibleDice`
  (`|SpawnActorFromClass` "/Game/_MainProject/Blueprints/Actors/Loot/Actor_Dice.Actor_Dice_C" (`KismetMathLibrary.MakeTransform` (550.0 0.0 110.0) (struct) (0.585 0.585 0.585)) "Undefined" "OverrideRootScale" null null null))

(event `EventGenerateStarterEquipment`
  (`self.GenerateStarterEquipment`))

(event `SpawnActor`
  (params (Actor :type "Actor Class Reference"))
  (`|SpawnActorFromClass` Actor (`KismetMathLibrary.MakeTransform` (550.0 0.0 110.0) (struct :`Yaw` 180.0) (0.585 0.585 0.585)) "Undefined" "OverrideRootScale" null null))

(fn `GenerateStarterEquipment`
  (locals (EquipmentDataTable :type "DataTable Object Reference" :default "DataTable'/Game/_MainProject/Blueprints/DataTables/StarterEquipmentDataTable.StarterEquipmentDataTable'") (Int :type Integer) (TmpEquipmentStrucuture :type "/Game/_MainProject/Blueprints/Structures/StructEquipment Structure") (EquipmentWidgetArray :type "Array of /Game/_MainProject/Blueprints/Widgets/Inventory/Equipment/EquipmentWidget Object Reference"))
  (bind _equipment (`/Game/_MainProject/Blueprints/FunctionLibrary.GetAllEquipmentFromRarity` "NewEnumerator4" self))
  (bind _asbp_player (cast `/Game/_MainProject/Blueprints/Actors/BP_Player` (`GameplayStatics.GetPlayerCharacter` 0)))
  (for _array_element _equipment
    (`/Game/_MainProject/Blueprints/Widgets/Inventory/InventorySpace.AddItem` (`/Game/_MainProject/Blueprints/Widgets/Inventory/Inventory.InactiveInventorySpace` (`/Game/_MainProject/Blueprints/Widgets/HUD.Inventory` (`/Game/_MainProject/Blueprints/Actors/BP_Player.HUD` _asbp_player))) _array_element)))

(fn `UserConstructionScript`)