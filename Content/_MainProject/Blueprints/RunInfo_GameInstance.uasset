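; RunInfo_GameInstance is a game instance that manages priority-ordered queues of widgets listening for input actions such as CloseWidget.
; Adding a widget appends it uniquely, then swaps it forward ahead of the first entry with equal or lower priority.
; It then calls stop-listening and re-enables listening only for the front of the CloseWidget queue.
; Removal takes a widget out and prints the result, without refreshing the listener.
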(fn `AddToListenQueue`
  (params (ListenQueue :type "Array of Widget Object Reference") (Priority :type Integer) (Widget :type "Widget Object Reference") (ActionName :type Name))
  (locals (TargetIndex :type Integer) (AddedIndex :type Integer) (ItemAdded :type Boolean))
  ;[1 1 1] Add First Item to Queue if empty
  (if (`KismetArrayLibrary.Array_IsValidIndex` ListenQueue)
    ;[1 1 1] Add new Widget to Listen Queue
    (for (_array_element _array_index) ListenQueue
      (bind _asuser_widget (cast `UserWidget` _array_element))
      (if (<= (`UserWidget.Priority` _asuser_widget) Priority)
        (set `local.TargetIndex` _array_index)
        (bind _returnvalue (`KismetArrayLibrary.Array_AddUnique` ListenQueue Widget))
        (set `local.AddedIndex` _returnvalue)
        (set `local.ItemAdded` true)
        (break)))
    ;[1 1 1] Add new Widget at last index to Listen Queue
    (if (not (`local.ItemAdded`))
      (bind _returnvalue_2 (`KismetArrayLibrary.Array_AddUnique` ListenQueue Widget))
      (bind _output_get (set `local.AddedIndex` _returnvalue_2))
      (set `local.TargetIndex` _output_get))
    ;[1 1 1] Swap Widgets in Queue to adjust Priority of new item
    (while (> (`local.AddedIndex`) (`local.TargetIndex`))
      (`KismetArrayLibrary.Array_Swap` ListenQueue (`local.AddedIndex`) (- (`local.AddedIndex`) 1))
      (`/Engine/EditorBlueprintResources/StandardMacros.DecrementInt` (`local.AddedIndex`)))
    (else
      (`KismetArrayLibrary.Array_AddUnique` ListenQueue Widget)))
  (`self.StopListening`) ; Stop All Items from Queue from Listening
  (`self.EnableListenFromQueue`))

(fn `EnableListenFromQueue`
  (bind _closewidgetlistenqueue (`self.CloseWidgetListenQueue`))
  (`|ExecutionSequence`
    (:`then_0`
      (if (`KismetArrayLibrary.Array_IsValidIndex` _closewidgetlistenqueue)
        (`self.StartListening` (`|GetArrayItem` _closewidgetlistenqueue) "CloseWidget")))))

(fn `RemoveFromListenQueue`
  (params (WidgetQueue :type "Array of Widget Object Reference") (`Target Widget` :type "Widget Object Reference"))
  (bind _returnvalue (`KismetArrayLibrary.Array_RemoveItem` WidgetQueue `Target Widget`))
  (if _returnvalue
    (`KismetSystemLibrary.PrintString` (`KismetTextLibrary.Conv_TextToString` (`|FormatText` "{Item} succesfully removed from Listen Queue" `Target Widget`)))
    (else
      (`KismetSystemLibrary.PrintString` (`KismetTextLibrary.Conv_TextToString` (`|FormatText` "{Item} removal failed from Listen Queue" `Target Widget`))))))